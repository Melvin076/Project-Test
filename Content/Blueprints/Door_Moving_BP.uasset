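; Sliding double-door actor for EWA-RPG that opens when anything overlaps its Box trigger and closes when the overlap ends.
; Two static mesh panels slide apart along local X by lerping their relative locations from timeline alphas.
; Opening and closing use separate timelines that always restart from their endpoints, with no check on the overlapping actor.
; BeginPlay prints a starter-door version string.
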(event OnComponentBeginOverlap(Box)
  (params (OverlappedComponent :type Primitive%20Component%20Object%20Reference) (OtherActor :type Actor%20Object%20Reference) (OtherComp :type Primitive%20Component%20Object%20Reference) (OtherBodyIndex :type Integer) (bFromSweep :type Boolean) (SweepResult :type Hit%20Result%20Structure%20%28by%20ref%29))
  (bind _alphavalue (Timeline|DoorOpening PlayFromStart)
    (:Update
      (Transformation|SetRelativeLocation (Variables|Default|GetStaticMesh) (Math|Vector|Lerp(Vector) "-55.312401, 0, 0" "-100.000000, 0, 0" _alphavalue) false false)
      (Transformation|SetRelativeLocation (Variables|Default|GetStaticMesh1) (Math|Vector|Lerp(Vector) "50.292953, 0, 0" "100.000000, 0, 0" _alphavalue) false false))))

(event OnComponentEndOverlap(Box)
  (params (OverlappedComponent :type Primitive%20Component%20Object%20Reference) (OtherActor :type Actor%20Object%20Reference) (OtherComp :type Primitive%20Component%20Object%20Reference) (OtherBodyIndex :type Integer))
  (bind _alphavalue (Timeline|Timeline_0 ReverseFromEnd)
    (:Update
      (Transformation|SetRelativeLocation (Variables|Default|GetStaticMesh) (Math|Vector|Lerp(Vector) "-55.312401, 0, 0" "-100.000000, 0, 0" _alphavalue) false false)
      (Transformation|SetRelativeLocation (Variables|Default|GetStaticMesh1) (Math|Vector|Lerp(Vector) "50.292953, 0, 0" "100.000000, 0, 0" _alphavalue) false false))))

(event EventBeginPlay
  (Development|PrintString "EWA-RPG StarterDoor V. 0.0.1"))

(event Collision|EventActorBeginOverlap
  (params (OtherActor :type Actor%20Object%20Reference)))

(event EventTick
  (params (DeltaSeconds :type Float%20%28single-precision%29)))

(fn ConstructionScript)